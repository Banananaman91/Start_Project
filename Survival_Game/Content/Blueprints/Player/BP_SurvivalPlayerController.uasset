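; BP_SurvivalPlayerController is a player controller that toggles the inventory screen through the OpenInventory input action.
; It creates a WBP_Inventory widget when no valid one exists, stores the reference and adds it to the viewport.
; Opening shows the mouse cursor and switches to Game and UI input mode focused on the widget.
; Pressing again while it is displayed calls the widget's own CloseInventory function.
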(event EventBeginPlay)

(event EventTick
  (params (DeltaSeconds :type Float%20%28single-precision%29)))

(event Input|ActionEvents|InputActionOpenInventory
  (params (Key :type Key%20Structure :default "None"))
  (:Pressed
    (Utilities|IsValid (Variables|Default|GetInventoryWidget)
      (:Is%20Valid
        (if (UserInterface|Viewport|IsinViewport (Variables|Default|GetInventoryWidget))
          (Default|CloseInventory (Variables|Default|GetInventoryWidget))
          (else
            (Utilities|IsValid 0
              (:Is%20Valid
                _)
              (:Is%20Not%20Valid
                (bind _returnvalue (UserInterface|CreateWidget "/Game/Blueprints/Widgets/WBP_Inventory.WBP_Inventory_C" :!label _label))
                (Variables|Default|SetInventoryWidget _returnvalue)))
            (UserInterface|Viewport|AddtoViewport (Variables|Default|GetInventoryWidget) 0)
            (Variables|Default|SetbShowMouseCursor true)
            (Input|SetInputModeGameandUI self (Variables|Default|GetInventoryWidget) "DoNotLock" true))))
      (:Is%20Not%20Valid
        (goto _label)))))

(fn ConstructionScript)